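; Actor component for a chain hook that grabs, carries and throws BP_ThrowableActor objects.
; It spawns a BP_Chain at BeginPlay; throwing extends it from below the camera.
; Looping timers move the chain and sphere-trace to its tip; a hit halts spawning, trims length and pins the mesh to the tip with physics off.
; Scrolling adds or removes links; stopping despawns the chain and releases the mesh with the tip's velocity.
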(event Custom|StartThrow
  (Default|SpawnChain (Variables|Workflow|GetChain))
  (Utilities|Time|SetTimerbyEvent (delegate Custom|UpdateStartPosition) (Variables|Throw|GetThrowDeltaTime) true)
  (Utilities|Time|SetTimerbyEvent (delegate Custom|ScanningForObjects) (Variables|Throw|GetThrowDeltaTime) true)
  (EventDispatchers|AssignOnChainSpawned (Variables|Workflow|GetChain) (delegate Custom|OnChainSpawned_Event)))

(event Custom|ScrollDistance
  (params (Value :type Float%20%28double-precision%29))
  ;[1 1 1] Distance control
  (if (> Value 0.0)
    (bind _chain (Variables|Workflow|GetChain)
      (:then
        (Default|AddChainElement _chain))
      (:else))
    (else
      (bind _chain_2 (Variables|Workflow|GetChain)
        (:then
          (Default|RemoveChainElement _chain_2))
        (:else)))))

(event Custom|ScanningForObjects
  (bind _chain (Variables|Workflow|GetChain))
  (bind _chainelements (Variables|/Game/Task_07/BP_Chain.BP_Chain_C|GetChainElements _chain))
  ;[0.276 0.276 0.276] ScanForObjects
  (bind (_outhit _returnvalue) (Collision|SphereTraceByChannel (Transformation|GetActorLocation (Components|GetOwner)) (Utilities|Array|Get(acopy) _chainelements (Utilities|Array|LastIndex _chainelements)) 1e+01 "TraceTypeQuery1" false 0 "None"))
  (if _returnvalue
    (bind _asbp_throwable_actor (Utilities|Casting|CastToBP_ThrowableActor (.HitActor (Collision|BreakHitResult _outhit)))
      (:then
        (Variables|Default|SetGrabbedActor (Variables|/Game/Task_07/BP_ThrowableActor.BP_ThrowableActor_C|GetABCDMesh _asbp_throwable_actor))
        (Default|InterruptSpawn (Variables|Workflow|GetChain) :!label _label)
        (Default|InteruptDespawn (Variables|Workflow|GetChain))
        (Utilities|Time|SetTimerbyEvent (delegate Custom|ScanningForObjects) -1.0)
        (Utilities|Time|SetTimerbyEvent (delegate Custom|UpdateGrabbedItemPos) (Variables|Throw|GetThrowDeltaTime) true)
        (Utilities|FlowControl|ForLoopwithBreak 0 100 :!label _label_2
          (:LoopBody
            (if (Math|Float|NearlyEqual(Float) (Math|Vector|Distance(Vector) (Transformation|GetActorLocation (Variables|Workflow|GetChain)) (Transformation|GetWorldLocation (Variables|Default|GetGrabbedActor))) (.ReturnValue (Default|GetChainLength (Variables|Workflow|GetChain))) 1e+02)
              (goto _label_2 Break)
              (else
                (Default|RemoveChainElement (Variables|Workflow|GetChain)))))))
      (:CastFailed
        (CallFunction|StopThrow)))
    (else
      (Utilities|IsValid (Variables|Default|GetGrabbedActor)
        (:Is%20Valid
          (goto _label))))))

(event Custom|UpdateStartPosition
  (bind _returnvalue (Game|GetPlayerCameraManager 0))
  (bind _returnvalue_2 (Transformation|GetActorTransform _returnvalue))
  ;[1 0 0] UpdateChainActorPos
  (Transformation|SetActorTransform (Variables|Workflow|GetChain) (Math|Transform|MakeTransform (+ (* (Transformation|GetActorUpVector (Game|GetPlayerCameraManager 0)) -7e+01) (.location _returnvalue_2)) (.rotation _returnvalue_2) (.scale _returnvalue_2))))

(event Custom|OnChainSpawned_Event
  (Utilities|FlowControl|Delay 0.5) ; Delay for better looks
  (Variables|Default|GetGrabbedActor
    (:then)
    (:else
      (CallFunction|StopThrow))))

(event Custom|UpdateGrabbedItemPos
  (CallFunction|UpdateMeshPosition))

(event Custom|StopThrow
  ;[1 1 1] Stop throw
  (Utilities|Time|SetTimerbyFunctionName 0 "UpdateGrabbedItemPos" -1.0)
  (Utilities|Time|SetTimerbyFunctionName 0 "ScanningForObjects" -1.0)
  (bind _chain (Variables|Workflow|GetChain)
    (:then
      (bind _grabbedactor (Variables|Default|GetGrabbedActor)
        (:then
          (Physics|SetSimulatePhysics _grabbedactor true)
          (Physics|SetPhysicsLinearVelocity _grabbedactor (Variables|/Game/Task_07/BP_Chain.BP_Chain_C|GetVelocity%20Of%20Last%20Element _chain) false "None"))
        (:else
          _))
      (Default|DespawnChain (Variables|Workflow|GetChain))
      (Variables|Default|SetGrabbedActor 0))
    (:else)))

(event EventBeginPlay
  ;[1 1 1] Chain spawn
  (bind _returnvalue (Game|SpawnActorfromClass "/Game/Task_07/BP_Chain.BP_Chain_C" (Math|Transform|MakeTransform (Utilities|GetStartPosition)) "AlwaysSpawn" "MultiplyWithRoot" 0 0))
  (Variables|Workflow|SetChain _returnvalue))

(fn AngleBetweenVectors
  (params (V1 :type Vector) (V2 :type Vector))
  (return (Class|KismetMathLibrary|DegAcos (Math|Vector|DotProduct V1 V2))))

(fn RotateVectortoVector
  (params (VectorToRotate :type Vector) (TargetVector :type Vector) (AngleDeg :type Float%20%28double-precision%29))
  (return (Math|Vector|RotateVectorAroundAxis VectorToRotate AngleDeg (Math|Vector|CrossProduct (+ VectorToRotate "0.001000,0.001000,0.001000") TargetVector))))

(fn UpdateMeshPosition
  (bind _chain (Variables|Workflow|GetChain))
  (bind _chainelements (Variables|/Game/Task_07/BP_Chain.BP_Chain_C|GetChainElements _chain))
  (bind _grabbedactor (Variables|Default|GetGrabbedActor)
    (:then
      (if (> (Math|Vector|Distance(Vector) (Transformation|GetWorldLocation (Variables|Default|GetGrabbedActor)) (|LastElementPosition)) 35.0)
        _
        (else
          _))
      (Physics|SetSimulatePhysics _grabbedactor false)
      (Transformation|SetWorldLocation _grabbedactor (Utilities|Array|Get(acopy) _chainelements (Utilities|Array|LastIndex _chainelements)) false false))
    (:else)))