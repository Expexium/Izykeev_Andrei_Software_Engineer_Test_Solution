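; Chain actor that extends and retracts one element at a time on looping timers, notifying when fully spawned.
; A straight template along the actor's forward vector is stored in local space and rebuilt on each length change.
; A fixed-interval timer eases each point toward its template offset from the previous point, creating trailing lag, then rebuilds the spline and its spline meshes.
; It also exposes chain length plus the last element's location and velocity.
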(event Custom|DefineChain
  (params (Elements :type Integer))
  ;[1 0.7389 0 1 26] Creating a chain
  (Utilities|Array|Clear (Variables|Chain|GetLocalSpaceOriginalChain))
  (bind _createdchain (CallFunction|CreateChain (Variables|ChainSettings|GetDistanceBetweenChainElements) Elements (Transformation|GetActorForwardVector) (Transformation|GetActorLocation)))
  (for _array_element _createdchain
    (Utilities|Array|Add (Variables|Chain|GetLocalSpaceOriginalChain) (Math|Transform|InverseTransformLocation (Transformation|GetActorTransform) _array_element))))

(event Custom|SetUpdateChainTimer
  (Utilities|Time|SetTimerbyEvent (delegate Custom|UpdateChain) (Variables|Default|GetChainGlobalDeltaTime) true))

(event Custom|InteruptDespawn
  ;[1 0.01418 0 1 82] Spawn and despawn
  (Utilities|Time|PauseTimerbyHandle (Variables|Timers|GetDespawnTimer)))

(event Custom|InterruptSpawn
  ;[1 0.01418 0 1 82] Spawn and despawn
  (Utilities|Time|PauseTimerbyHandle (Variables|Timers|GetSpawnTimer)))

(event Custom|UpdateChain
  (bind _chainelements (Variables|Chain|GetChainElements))
  ;[0.3229 0.153 0] Adding Chain Length depending on LocalSpaceOriginalChain
  (for (_ _array_index) (Variables|Chain|GetLocalSpaceOriginalChain)
    (if (not (Utilities|Array|IsValidIndex _chainelements _array_index))
      (Utilities|Array|Insert _chainelements (Transformation|GetActorLocation))))
  ;[1 0 0.04709] Deleting Chain elements depending on LocalSpaceOriginalChain
  (for _index (range 1 (- (Utilities|Array|Length (Variables|Chain|GetChainElements)) (Utilities|Array|Length (Variables|Chain|GetLocalSpaceOriginalChain))))
    (Utilities|Array|RemoveIndex (Variables|Chain|GetChainElements)))
  ;[0.06266 0.2447 0.3646] Workflow
  (if (> (Utilities|Array|Length (Variables|Chain|GetLocalSpaceOriginalChain)) 0)
    (bind _velocityoflastelement (CallFunction|ChainMovement (Variables|Chain|GetChainElements) (Variables|ChainSettings|GetDelayPerElement) (Variables|Default|GetChainGlobalDeltaTime) (Variables|Chain|GetLocalSpaceOriginalChain) (Transformation|GetActorTransform)))
    (Variables|Default|SetVelocity%20Of%20Last%20Element _velocityoflastelement)
    (Spline|SetSplinePoints (Variables|Default|GetSpline) (Variables|Chain|GetChainElements) "World" true)
    (CallFunction|UpdateSplineMesh)))

(event Custom|RemoveChainElement
  ;[0.1562 0.1562 0.1562] Manipulating Elements
  (CallFunction|DefineChain (- (Utilities|Array|Length (Variables|Chain|GetLocalSpaceOriginalChain)) 1)))

(event Custom|AddChainElement
  ;[0.1562 0.1562 0.1562] Manipulating Elements
  (CallFunction|DefineChain (+ (Utilities|Array|Length (Variables|Chain|GetLocalSpaceOriginalChain)) 1)))

(event Custom|SpawnChain
  ;[1 0.01418 0 1 82] Spawn and despawn
  (Utilities|Time|PauseTimerbyHandle (Variables|Timers|GetDespawnTimer))
  (Utilities|Time|UnpauseTimerbyHandle (Variables|Timers|GetSpawnTimer))
  (if (< (Utilities|Array|Length (Variables|Chain|GetLocalSpaceOriginalChain)) (Variables|ChainSettings|GetMaxElements))
    (CallFunction|AddChainElement)
    (else
      (Utilities|Time|PauseTimerbyHandle (Variables|Timers|GetSpawnTimer))
      (Default|CallOnChainSpawned))))

(event Custom|DespawnChain
  ;[1 0.01418 0 1 82] Spawn and despawn
  (Utilities|Time|PauseTimerbyHandle (Variables|Timers|GetSpawnTimer))
  (Utilities|Time|UnpauseTimerbyHandle (Variables|Timers|GetDespawnTimer))
  (if (> (Utilities|Array|Length (Variables|Chain|GetLocalSpaceOriginalChain)) 0)
    (CallFunction|RemoveChainElement)
    (else
      (Utilities|Time|PauseTimerbyHandle (Variables|Timers|GetDespawnTimer)))))

(event EventBeginPlay
  ;[1 0.01418 0 1 82] Spawn and despawn
  (Utilities|FlowControl|Delay 0.2)
  (bind _returnvalue (Utilities|Time|SetTimerbyEvent (delegate Custom|DespawnChain) 0.05 true))
  (bind _output_get (Variables|Timers|SetDespawnTimer _returnvalue))
  (Utilities|Time|PauseTimerbyHandle _output_get)
  (bind _returnvalue_2 (Utilities|Time|SetTimerbyEvent (delegate Custom|SpawnChain) 0.02 true))
  (bind _output_get_2 (Variables|Timers|SetSpawnTimer _returnvalue_2))
  (Utilities|Time|PauseTimerbyHandle _output_get_2)
  (CallFunction|SetUpdateChainTimer))

(fn ConstructionScript)

(fn CreateChain
  (params (DistanceBetweenChainElements :type Float%20%28double-precision%29) (Elements :type Integer) (Direction :type Vector) (StartLocation :type Vector))
  (if (> Elements 0)
    (Utilities|Array|Add (LocalVariables|GetChain) StartLocation)
    (for _index (range 0 (- Elements 2))
      (Utilities|Array|Add (LocalVariables|GetChain) (+ (Utilities|Array|Get(acopy) (LocalVariables|GetChain) _index) (* Direction DistanceBetweenChainElements))))
    (return (LocalVariables|GetChain))))

(fn ChainMovement
  (params (Chain :type Array%20of%20Vectors) (DelayPerElement :type Float%20%28double-precision%29) (DeltaTime :type Float%20%28double-precision%29) (OriginalChainLocalSpace :type Array%20of%20Vectors) (ActorTransform :type Transform))
  (for (_ _array_index) OriginalChainLocalSpace
    (if (== _array_index (Utilities|Array|LastIndex Chain))
      (LocalVariables|SetLastElVel (* (Math|Vector|GetUnitDirection(Vector) (Utilities|Array|Get(acopy) Chain _array_index) (Math|Vector|SelectVector (|PerfectLocationCalculation _array_index) (Math|Transform|TransformLocation ActorTransform (Utilities|Array|Get(acopy) OriginalChainLocalSpace)) (> _array_index 0))) (/ (Math|Vector|Distance(Vector) (Math|Vector|SelectVector (|PerfectLocationCalculation _array_index) (Math|Transform|TransformLocation ActorTransform (Utilities|Array|Get(acopy) OriginalChainLocalSpace)) (> _array_index 0)) (Utilities|Array|Get(acopy) Chain _array_index)) DelayPerElement))))
    (Utilities|Array|SetArrayElem Chain _array_index (+ (Utilities|Array|Get(acopy) Chain _array_index) (Math|Vector|ClampVectorSize (* (Math|Vector|GetUnitDirection(Vector) (Utilities|Array|Get(acopy) Chain _array_index) (Math|Vector|SelectVector (|PerfectLocationCalculation _array_index) (Math|Transform|TransformLocation ActorTransform (Utilities|Array|Get(acopy) OriginalChainLocalSpace)) (> _array_index 0))) (* (/ (Math|Vector|Distance(Vector) (Math|Vector|SelectVector (|PerfectLocationCalculation _array_index) (Math|Transform|TransformLocation ActorTransform (Utilities|Array|Get(acopy) OriginalChainLocalSpace)) (> _array_index 0)) (Utilities|Array|Get(acopy) Chain _array_index)) DelayPerElement) DeltaTime)) 0.0 (Math|Vector|Distance(Vector) (Math|Vector|SelectVector (|PerfectLocationCalculation _array_index) (Math|Transform|TransformLocation ActorTransform (Utilities|Array|Get(acopy) OriginalChainLocalSpace)) (> _array_index 0)) (Utilities|Array|Get(acopy) Chain _array_index))))))
  (return (LocalVariables|GetLastElVel)))

(fn UpdateSplineMesh
  (bind _splinemeshcomponents (Variables|Chain|GetSplineMeshComponents))
  (bind _spline (Variables|Default|GetSpline))
  (bind _spline_2 (Variables|Default|GetSpline))
  (bind _returnvalue (Utilities|Array|LastIndex _splinemeshcomponents))
  (for _index (range 1 (- (Utilities|Array|Length (Variables|Chain|GetSplineMeshComponents)) (Utilities|Array|Length (Variables|Chain|GetLocalSpaceOriginalChain))))
    (Components|DestroyComponent (Utilities|Array|Get(acopy) _splinemeshcomponents _returnvalue))
    (Utilities|Array|RemoveIndex _splinemeshcomponents _returnvalue))
  (for _index_2 (range 0 (- (Spline|GetNumberOfSplinePoints (Variables|Default|GetSpline)) 1))
    (Utilities|IsValid (Utilities|Array|Get(acopy) (Variables|Chain|GetSplineMeshComponents) _index_2)
      (:Is%20Valid
        _)
      (:Is%20Not%20Valid
        (bind _returnvalue_2 (AddComponent|AddSplineMeshComponent true))
        (Collision|SetCollisionResponsetoAllChannels _returnvalue_2 "ECR_Ignore")
        (Utilities|Array|Add (Variables|Chain|GetSplineMeshComponents) _returnvalue_2)
        (Transformation|SetMobility _returnvalue_2 "Movable")
        (SplineMesh|SetForwardAxis _returnvalue_2 "Z" true)
        (Components|StaticMesh|SetStaticMesh _returnvalue_2 (Variables|Chain|GetMesh))
        (Transformation|AttachComponentToComponent _returnvalue_2 (Variables|Default|GetSpline) "None" "KeepRelative" "KeepRelative" "KeepRelative" true)))
    (SplineMesh|SetStartandEnd (Utilities|Array|Get(acopy) (Variables|Chain|GetSplineMeshComponents) _index_2) (Spline|GetLocationatSplinePoint _spline _index_2 "Local") (Spline|GetTangentatSplinePoint _spline _index_2 "Local") (Spline|GetLocationatSplinePoint _spline_2 (+ _index_2 1) "Local") (Spline|GetTangentatSplinePoint _spline_2 (+ _index_2 1) "Local") true :!class /Script/Engine.SplineMeshComponent)))

(fn GetChainLength
  (bind _distancebetweenchainelements (Variables|ChainSettings|GetDistanceBetweenChainElements))
  (return (* (Utilities|Array|Length (Variables|Chain|GetLocalSpaceOriginalChain)) _distancebetweenchainelements) _distancebetweenchainelements))

(fn GetLastChainElementLocation
  (bind _chainelements (Variables|Chain|GetChainElements))
  (return (Utilities|Array|Get(acopy) _chainelements (Utilities|Array|LastIndex _chainelements))))