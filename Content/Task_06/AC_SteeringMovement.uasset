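; Steering movement component that flies its owner forward at max speed, turning toward a target actor or location at a capped rate per second.
; Each tick it predicts the turning arc in steps and sphere-traces the segments for obstacles.
; A hit flag selects between homing and UpperMovement avoidance, but a trace hit sets it false and UpperMovement's vertical-dodge math is unconnected, so avoidance looks unfinished.
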(event EventTick
  (params (DeltaSeconds :type Float%20%28single-precision%29))
  (Variables|Default|SetCurrentMovementSpeed (Variables|Default|GetMaxMovementSpeed))
  (bind (_hit _outhit) (CallFunction|CalculateTrajectory (Variables|Default|GetTrajectorySteps) (Transformation|GetActorLocation (Components|GetOwner))))
  (Transformation|SetActorRotation (Components|GetOwner) (Math|Conversions|RotationFromXVector (Math|Vector|SelectVector (|UpperMovement _outhit) (CallFunction|RotateVectortoVector (Transformation|GetActorForwardVector (Components|GetOwner)) (Math|Vector|GetUnitDirection(Vector) (Transformation|GetActorLocation (Components|GetOwner)) (CallFunction|GetRealTargetLocation)) (CallFunction|AngletoRotate (Utilities|Time|GetWorldDeltaSeconds))) _hit)))
  (Transformation|AddActorWorldOffset (Components|GetOwner) (* (Variables|Default|GetCurrentMovementSpeed) (Utilities|Time|GetWorldDeltaSeconds) (Transformation|GetActorForwardVector (Components|GetOwner)))))

(fn AngleBetweenVectors
  (params (V1 :type Vector) (V2 :type Vector))
  (return (Class|KismetMathLibrary|DegAcos (Math|Vector|DotProduct V1 V2))))

(fn RotateVectortoVector
  (params (VectorToRotate :type Vector) (TargetVector :type Vector) (AngleDeg :type Float%20%28double-precision%29))
  (return (Math|Vector|RotateVectorAroundAxis VectorToRotate AngleDeg (Math|Vector|CrossProduct (+ VectorToRotate "0.001000,0.001000,0.001000") TargetVector))))

(fn GetRealTargetLocation
  (Utilities|IsValid (Variables|Target|GetTargetActor)
    (:Is%20Valid
      (return (Transformation|GetActorLocation (Variables|Target|GetTargetActor))))
    (:Is%20Not%20Valid
      (return (Variables|Target|GetTargetLocation)))))

(fn AngletoRotate
  (params (DeltaTime :type Float%20%28double-precision%29))
  (bind _returnvalue (Components|GetOwner))
  (bind _targetloc (CallFunction|GetRealTargetLocation))
  (bind _returnvalue_2 (Components|GetOwner))
  (bind _returnvalue_3 (Transformation|GetActorForwardVector _returnvalue))
  (bind _returnvalue_4 (Transformation|GetActorLocation _returnvalue_2))
  (bind _returnvalue_5 (Math|Vector|GetUnitDirection(Vector) _returnvalue_4 _targetloc))
  (bind _angle (CallFunction|AngleBetweenVectors _returnvalue_5 _returnvalue_3))
  (return (- _angle (Math|Float|Clamp(Float) (- _angle (* (Variables|Default|GetRotationPerSecond) DeltaTime)) 0.0 9999.0))))

(fn CalculateTrajectory
  (params (Steps :type Integer) (StartLocation :type Vector))
  (LocalVariables|SetDeltaTime (/ 1.0 (/ (Math|Conversions|ToFloat(Integer) Steps) (/ 9e+01 (Variables|Default|GetRotationPerSecond)))))
  (LocalVariables|SetLastForwardVector (Transformation|GetActorForwardVector (Components|GetOwner)))
  (Utilities|Array|Add (LocalVariables|GetTrajectory) StartLocation)
  (bind _index (Utilities|FlowControl|ForLoopwithBreak 1 Steps :!label _label)
    (:LoopBody
      ;[1 0.3159 0] Next Element
      (Utilities|Array|Add (LocalVariables|GetTrajectory) (+ (CallFunction|CalculateDeltaVelocity (LocalVariables|GetLastForwardVector) (LocalVariables|GetDeltaTime) 1.0) (Utilities|Array|Get(acopy) (LocalVariables|GetTrajectory) (- _index 1))))
      (LocalVariables|SetLastForwardVector (Math|Vector|Normalize (CallFunction|CalculateDeltaVelocity (LocalVariables|GetLastForwardVector) (LocalVariables|GetDeltaTime) 1.0)))
      (if (!= (- _index 1) 0)
        (bind (_outhit _returnvalue) (Collision|SphereTraceByChannel (Utilities|Array|Get(acopy) (LocalVariables|GetTrajectory) (- _index 1)) (Utilities|Array|Get(acopy) (LocalVariables|GetTrajectory) _index) 3e+01 "TraceTypeQuery1" false 0 "None"))
        (if _returnvalue
          (LocalVariables|SetWasHit false)
          (goto _label Break))))
    (:Completed
      (return (LocalVariables|GetWasHit) _outhit))))

(fn CalculateDeltaVelocity
  (params (ForwardVector :type Vector) (DeltaTime :type Float%20%28double-precision%29) (AngleMultiplier :type Float%20%28double-precision%29))
  (return (* (CallFunction|RotateVectortoVector ForwardVector (Math|Vector|GetUnitDirection(Vector) (Transformation|GetActorLocation (Components|GetOwner)) (CallFunction|GetRealTargetLocation)) (* (CallFunction|AngletoRotate DeltaTime) AngleMultiplier)) (Variables|Default|GetMaxMovementSpeed) DeltaTime)))