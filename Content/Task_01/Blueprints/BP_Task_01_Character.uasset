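; Player character Blueprint for Task 01 that lets the player interact with actors in front of the camera.
; When IA_Interact starts, ForwardLineTrace casts a Visibility line from the player camera manager along its forward vector, up to a configurable distance.
; On a hit, the character calls OnInteractionMessage on the hit actor, passing itself, so each target handles its own response.
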(event Input|EnhancedActionEvents|EnhancedInputActionIA_Interact
  (params (ActionValue :type Boolean) (ElapsedSeconds :type Float%20%28double-precision%29) (TriggeredSeconds :type Float%20%28double-precision%29) (InputAction :type Input%20Action%20Object%20Reference :default "/Game/Basic/Input/IA_Interact.IA_Interact"))
  ;[1 1 1] Didnt touch BPC_Input
  (:Started
    (bind (_washit _outhit) (CallFunction|ForwardLineTrace))
    (if _washit
      (Class|BPIInteraction|OnInteraction(Message) (.HitActor (Collision|BreakHitResult _outhit)) self))))

(event EventBeginPlay)

(fn ConstructionScript)

(fn ForwardLineTrace
  (bind _returnvalue (Game|GetPlayerCameraManager 0))
  (bind _returnvalue_2 (Transformation|GetActorLocation _returnvalue))
  (bind (_outhit _returnvalue_3) (Collision|LineTraceByChannel _returnvalue_2 (+ _returnvalue_2 (* (Transformation|GetActorForwardVector _returnvalue) (Variables|Default|GetInteractionTraceFromCameraDistance))) "TraceTypeQuery1" false 0 "None"))
  (return _returnvalue_3 _outhit))