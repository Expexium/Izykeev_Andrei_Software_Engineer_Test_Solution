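; Blueprint function library whose CanInteractWith check decides whether Who can interact with a target actor, With.
; A Visibility trace from With to Who, ignoring With, must hit Who to confirm a clear line between them.
; A second trace 600 units along player 0's camera forward vector must then hit With, so the target has to be aimed at and within reach.
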(fn CanInteractwith
  (params (Who :type Actor%20Object%20Reference) (With :type Actor%20Object%20Reference))
  (bind _returnvalue (Game|GetPlayerCameraManager 0))
  (bind _returnvalue_2 (Transformation|GetActorLocation _returnvalue))
  (bind _outhit (Collision|LineTraceByChannel 0 (Transformation|GetActorLocation With) (Transformation|GetActorLocation Who) "TraceTypeQuery1" false (Utilities|Array|MakeArray With) "None" false))
  (if (== (.HitActor (Collision|BreakHitResult _outhit)) Who)
    (bind _outhit_2 (Collision|LineTraceByChannel 0 _returnvalue_2 (+ _returnvalue_2 (* (Transformation|GetActorForwardVector _returnvalue) 6e+02)) "TraceTypeQuery1" false 0 "None" false))
    (if (.bblockinghit _outhit_2)
      (return (== (.hitactor _outhit_2) With))
      (else
        (return false)))
    (else
      (return false))))