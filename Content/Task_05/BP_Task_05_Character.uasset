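; BP_Task_05_Character is a character that travels along a spline in a loop and throws balls with a chargeable force.
; BeginPlay caches the spline from SplineForMovement, then Tick advances a wrapped distance and teleports the character to that point's XY, keeping its own Z.
; Input adjusts the non-negative spline speed.
; Holding throw builds force on ACBallThrow and shows the trajectory, while release throws and resets the force.
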(event Input|EnhancedActionEvents|EnhancedInputActionIA_SplineMovementSpeedControl
  (params (ActionValue :type Float%20%28double-precision%29) (ElapsedSeconds :type Float%20%28double-precision%29) (TriggeredSeconds :type Float%20%28double-precision%29) (InputAction :type Input%20Action%20Object%20Reference :default "/Game/Basic/Input/Task5/IA_SplineMovementSpeedControl.IA_SplineMovementSpeedControl"))
  (Variables|Default|SetSplineMovementSpeed (Math|Float|Clamp(Float) (+ (* ActionValue 1e+03 (stale EventTick DeltaSeconds)) (Variables|Default|GetSplineMovementSpeed)) 0.0 99999999.0)))

(event Input|EnhancedActionEvents|EnhancedInputActionIA_ThrowBall
  (params (ActionValue :type Boolean) (ElapsedSeconds :type Float%20%28double-precision%29) (TriggeredSeconds :type Float%20%28double-precision%29) (InputAction :type Input%20Action%20Object%20Reference :default "/Game/Basic/Input/Task5/IA_ThrowBall.IA_ThrowBall"))
  (bind _ac_ballthrow (Variables|Default|GetAC_BallThrow))
  (:Triggered
    (Variables|/Game/Task_05/AC_BallThrow.AC_BallThrow_C|SetThrowForce _ac_ballthrow (+ (Variables|/Game/Task_05/AC_BallThrow.AC_BallThrow_C|GetThrowForce _ac_ballthrow) (* (Utilities|Time|GetWorldDeltaSeconds) 1e+03)))
    (Default|ShowTrajectory (Variables|Default|GetAC_BallThrow)))
  (:Completed
    (Default|Throw (Variables|Default|GetAC_BallThrow))
    (Variables|/Game/Task_05/AC_BallThrow.AC_BallThrow_C|SetThrowForce (Variables|Default|GetAC_BallThrow) 1e+02)))

(event EventBeginPlay
  (|GettingSpline) ; If invalid will stop doing anything
)

(event EventTick
  (params (DeltaSeconds :type Float%20%28single-precision%29))
  (bind _actualspline (Variables|Spline|GetActualSpline)
    (:then
      (bind _output_get (Variables|Default|SetCurrentDistanceOnSpline (Class|KismetMathLibrary|FWrap (+ (Variables|Default|GetCurrentDistanceOnSpline) (* (Variables|Default|GetSplineMovementSpeed) DeltaSeconds)) 0.0 (Spline|GetSplineLength _actualspline))))
      (Transformation|SetActorLocation (Math|Vector|MakeVector (.x (Spline|GetLocationatDistanceAlongSpline (Variables|Spline|GetActualSpline) _output_get "World")) (.y (Spline|GetLocationatDistanceAlongSpline (Variables|Spline|GetActualSpline) _output_get "World")) (.z (Transformation|GetActorLocation))) false true))
    (:else)))

(fn ConstructionScript)