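; Actor component that throws a physics ball from its owner along the instigator controller's forward vector and previews the flight path.
; On BeginPlay it spawns a hit-place marker; Throw spawns the ball and sets its launch velocity from ThrowForce.
; ShowTrajectory moves the marker to the predicted impact and draws debug spheres along the path.
; CalculateTrajectory integrates gravity in fixed time steps, line tracing each segment until a hit or point limit.
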(event Custom|ShowTrajectory
  (bind _returnvalue (Components|GetOwner))
  (bind (_trajectory _groundhit) (CallFunction|CalculateTrajectory (Transformation|GetActorLocation _returnvalue) (* (Variables|Default|GetThrowForce) (Transformation|GetActorForwardVector (Pawn|GetController (Variables|/Script/Engine.Actor|GetInstigator _returnvalue)))) 0.04 500 1e+02))
  (Transformation|SetActorLocation (Variables|Default|GetHitPlace) _groundhit false false)
  (for _array_element _trajectory
    (Rendering|Debug|DrawDebugSphere _array_element 1e+01 12 "(R=1.000000,G=0.040468,B=0.000000,A=1.000000)" 0.0)))

(event Custom|Throw
  (bind _returnvalue (Components|GetOwner))
  (bind _returnvalue_2 (Transformation|GetActorTransform _returnvalue))
  (bind _returnvalue_3 (Game|SpawnActorfromClass "/Game/Task_05/BP_PhysicBall.BP_PhysicBall_C" (Math|Transform|MakeTransform (.location _returnvalue_2) (.rotation _returnvalue_2) "1.000000,1.000000,1.000000") "Undefined" "MultiplyWithRoot" 0 0))
  (Physics|SetPhysicsLinearVelocity (Variables|/Game/Task_05/BP_PhysicBall.BP_PhysicBall_C|GetSphere _returnvalue_3) (* (Variables|Default|GetThrowForce) (Transformation|GetActorForwardVector (Pawn|GetController (Variables|/Script/Engine.Actor|GetInstigator (Components|GetOwner)))) 1.0) false "None"))

(event EventBeginPlay
  (bind _returnvalue (Game|SpawnActorfromClass "/Game/Task_05/BP_HitPlace.BP_HitPlace_C" (Math|Transform|MakeTransform "0, 0, 0" "0, 0, 0" "1.000000,1.000000,1.000000") "Undefined" "MultiplyWithRoot" 0 0))
  (Variables|Default|SetHitPlace _returnvalue))

(fn CalculateTrajectory
  (params (StartPosition :type Vector) (StartVelocity :type Vector) (DeltaTime :type Float%20%28double-precision%29) (MaxPossibleTrajectoryPoints :type Integer) (Mass :type Float%20%28double-precision%29))
  (Utilities|Array|Add (LocalVariables|GetAllTrajectoryPoints) StartPosition)
  (LocalVariables|SetLastTimeVelocity StartVelocity)
  (bind _index (Utilities|FlowControl|ForLoopwithBreak 1 MaxPossibleTrajectoryPoints :!label _label)
    (:LoopBody
      (Utilities|Array|Add (LocalVariables|GetAllTrajectoryPoints) (+ (Utilities|Array|Get(acopy) (LocalVariables|GetAllTrajectoryPoints) (- _index 1)) (* (+ (* (/ (+ (* (* Mass 9.8e+02) "0.000000,0.000000,-1.000000") (Math|Vector|MakeVector 0.0 0.0 0.0)) Mass) DeltaTime) (LocalVariables|GetLastTimeVelocity)) DeltaTime)))
      (LocalVariables|SetLastTimeVelocity (+ (* (/ (+ (* (* Mass 9.8e+02) "0.000000,0.000000,-1.000000") (Math|Vector|MakeVector 0.0 0.0 0.0)) Mass) DeltaTime) (LocalVariables|GetLastTimeVelocity)))
      (bind (_outhit _returnvalue) (Collision|LineTraceByChannel (Utilities|Array|Get(acopy) (LocalVariables|GetAllTrajectoryPoints) (- _index 1)) (Utilities|Array|Get(acopy) (LocalVariables|GetAllTrajectoryPoints) _index) "TraceTypeQuery1" false (Utilities|Array|MakeArray (Components|GetOwner)) "None"))
      (if _returnvalue
        (LocalVariables|SetHitGroundPoint (.ImpactPoint (Collision|BreakHitResult _outhit)))
        (goto _label Break)))
    (:Completed
      (return (LocalVariables|GetAllTrajectoryPoints) (LocalVariables|GetHitGroundPoint)))))